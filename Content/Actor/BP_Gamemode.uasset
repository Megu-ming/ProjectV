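; Game mode for a survival game that tracks XP, levels, kills and time-based difficulty, and creates the HUD.
; Enemy kills grant XP, and each level-up scales the next threshold and pauses the game to show a random pick of distinct augments.
; The chosen augment is applied to the player character, then leveled in the available pool and removed once it reaches max level.
; Event dispatchers broadcast XP, level and kill changes.
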(event `self.ReceiveBeginPlay`
  ; 위젯 생성
  (bind _returnvalue (`|CreateWidget` "/Game/Actor/UI/WBP_HUD.WBP_HUD_C" (`GameplayStatics.GetPlayerController` 0)))
  (`UserWidget.AddToViewport` _returnvalue 0)
  ; 초기화
  (set `self.Level` 1)
  (set `self.CurrentXp` 0.0)
  (set `self.NextLevelXp` (`self.BaseNextLevelXp`))
  (`self.OnXpChanged` (`self.CurrentXp`) (`self.NextLevelXp`))
  (`self.OnLevelUp` (`self.Level`))
  (set `self.AvailableAugment` (`self.AugmentList`)))

(event `self.ReceiveTick`
  (params (DeltaSeconds :type "Float (single-precision)"))
  ; 난이도 계산
  (bind _output_get (set `self.SurvivalTime` (+ DeltaSeconds (`self.SurvivalTime`))))
  (set `self.DifficultyLevel` (`KismetMathLibrary.FFloor` (/ _output_get (`self.DifficultyStepSeconds`)))))

(event `ApplyAugmentToPlayer`
  (params (SelectedData :type "/Game/Actor/Data/ST_AugmentData Structure"))
  (bind (_id _type _nametext _description _icon _value _level _maxlevel) (break `/Game/Actor/Data/ST_AugmentData` SelectedData))
  (bind (_item_id _item_type _item_nametext _item_description _item_icon _item_value _item_level _item_maxlevel) (break `/Game/Actor/Data/ST_AugmentData` (`self.Item`)))
  ; 증강 선택
  (bind _asbp_player (cast `/Game/Actor/BP_Character` (`GameplayStatics.GetPlayerCharacter` 0)))
  (`/Game/Actor/BP_Character.ApplyAugment` _asbp_player SelectedData)
  (`|ExecutionSequence`
    (:`then_0`
      (`GameplayStatics.SetGamePaused` false)
      (set `PlayerController.bShowMouseCursor` false (`self.PlayerController`))
      (`WidgetBlueprintLibrary.SetInputMode_GameOnly` (`self.PlayerController`)))
    (:`then_1`
      (for _index (range (`KismetArrayLibrary.Array_Length` (`self.AvailableAugment`)))
        (bind _output_id (break `/Game/Actor/Data/ST_AugmentData` (`|GetArrayItem` (`self.AvailableAugment`) _index)))
        (if (== _id _output_id)
          (set `self.NewLevel` (+ _level 1))
          (bind _output_get (set `self.Item` (make `/Game/Actor/Data/ST_AugmentData` _id _type _nametext _description _icon _value (`self.NewLevel`) _maxlevel)))
          (`KismetArrayLibrary.Array_Set` (`self.AvailableAugment`) _index _output_get)
          (if (>= _item_level _item_maxlevel)
            (`KismetArrayLibrary.Array_Remove` (`self.AvailableAugment`) _index)))))))

(fn `AddXp`
  (params (Amount :type "Float (double-precision)"))
  (bind _output_get (set `self.CurrentXp` (+ Amount (`self.CurrentXp`))))
  (`self.OnXpChanged` _output_get (`self.NextLevelXp`))
  (if (>= (`self.CurrentXp`) (`self.NextLevelXp`))
    (set `self.CurrentXp` (- (`self.CurrentXp`) (`self.NextLevelXp`)))
    (`self.LevelUp`)
    (`self.OnXpChanged` (`self.CurrentXp`) (`self.NextLevelXp`))))

(fn `EnemyKilled`
  (params (Amount :type Integer))
  (bind _output_get (set `self.KillCount` (+ Amount (`self.KillCount`))))
  (`self.OnKillCountChanged` _output_get)
  (`self.AddXp` 50.0))

(fn `GetRandomAugment`
  (params (Count :type Integer))
  (returns (Augment :type "Array of /Game/Actor/Data/ST_AugmentData Structure"))
  (locals (TempPool :type "Array of /Game/Actor/Data/ST_AugmentData Structure") (Result :type "Array of /Game/Actor/Data/ST_AugmentData Structure") (RandomIndex :type Integer :default 0))
  (bind _temppool (`local.TempPool`))
  (set `local.TempPool` (`self.AvailableAugment`))
  (for _ (range Count)
    (if (> (`KismetArrayLibrary.Array_Length` (`local.TempPool`)) 0)
      (set `local.RandomIndex` (`KismetMathLibrary.RandomIntegerInRange` 0 (- (`KismetArrayLibrary.Array_Length` _temppool) 1)))
      (`KismetArrayLibrary.Array_Add` (`local.Result`) (`|GetArrayItem` _temppool (`local.RandomIndex`)))
      (`KismetArrayLibrary.Array_Remove` (`local.TempPool`) (`local.RandomIndex`))
      (else
        (break))))
  (return (`local.Result`)))

(fn `LevelUp`
  (`/Engine/EditorBlueprintResources/StandardMacros.IncrementInt` (`self.Level`)
    (:`  `
      (set `self.NextLevelXp` (* (`self.NextLevelXp`) (`self.NextLevelXpMultiplier`)))
      (`self.OnLevelUp` (`self.Level`))
      (`self.ShowAugmentUI`))))

(fn `ShowAugmentUI`
  (if (== (`KismetArrayLibrary.Array_Length` (`self.AvailableAugment`)) 0)
    (return)
    (else
      (bind _augment (`self.GetRandomAugment` 3))
      (bind _returnvalue (`|CreateWidget` "/Game/Actor/UI/WBP_AugmentSelect.WBP_AugmentSelect_C" null _augment))
      (bind _output_get (set `self.AugmentUI` _returnvalue))
      (`UserWidget.AddToViewport` _output_get 0)
      (bind _output_get_2 (set `self.PlayerController` (`GameplayStatics.GetPlayerController` 0)))
      (set `PlayerController.bShowMouseCursor` true _output_get_2)
      (`GameplayStatics.SetGamePaused` true)
      (`WidgetBlueprintLibrary.SetInputMode_UIOnlyEx` (`self.PlayerController`) (`self.AugmentUI`)))))

(fn `UserConstructionScript`)