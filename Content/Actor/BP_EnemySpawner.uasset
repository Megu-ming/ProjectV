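; Enemy spawner that places pooled enemies around the player, scaling the alive cap with the game mode's difficulty.
; BeginPlay pre-spawns hidden, non-ticking, collision-free enemies and starts a looping SpawnLoop timer.
; When below the cap, each loop reactivates and resets one hidden enemy at a random offset from the player; the computed SpawnCount is unused.
; OnEnemyReturned reports the kill to BP_Gamemode and lowers the alive count.
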(event `self.ReceiveBeginPlay`
  ; Player Ref Setting
  (bind _asbp_character (cast `/Game/Actor/BP_Character` (`GameplayStatics.GetPlayerCharacter` 0)))
  (set `self.PlayerRef` _asbp_character)
  ; 생성한 적 오브젝트 풀에 등록
  (for _ (range (`self.InitialPoolSize`))
    (bind _returnvalue (`|SpawnActorFromClass` (`self.EnemyClass`) (`KismetMathLibrary.MakeTransform` (0.0 0.0 0.0)) "AlwaysSpawn" "MultiplyWithRoot" null null))
    (set `/Game/Actor/Enemy/BP_Enemy.SpawnerRef` self _returnvalue)
    (`KismetArrayLibrary.Array_Add` (`self.EnemyPool`) _returnvalue)
    (`self.SetActorHiddenInGame` _returnvalue true)
    (`self.SetActorTickEnabled` _returnvalue false)
    (`PrimitiveComponent.SetCollisionEnabled` (`Character.CapsuleComponent` _returnvalue) "NoCollision")
    ; 적 생성 타이머
    (`KismetSystemLibrary.K2_SetTimer` null "SpawnLoop" (`self.BaseSpawnInterval`) true)))

(event `OnEnemyReturned`
  ; 적이 죽었다면 KillCount 증가
  (bind _asbp_gamemode (cast `/Game/Actor/BP_Gamemode` (`GameplayStatics.GetGameMode`)))
  (`/Game/Actor/BP_Gamemode.EnemyKilled` _asbp_gamemode 1)
  (`/Engine/EditorBlueprintResources/StandardMacros.DecrementInt` (`self.AliveEnemy`)))

(fn `SpawnLoop`
  (locals (AvailableEnemy :type "/Game/Actor/Enemy/BP_Enemy Object Reference") (CurrentDifficulty :type Integer :default 0) (CurrentMaxAlive :type Integer) (SpawnCount :type Integer))
  (bind _availableenemy (`local.AvailableEnemy`))
  (bind (_returnvalue_x _returnvalue_y) (`KismetMathLibrary.BreakVector` (* (`KismetMathLibrary.RandomUnitVector`) (`self.SpawnRadius`))))
  ; 현재 난이도 캐싱 & 변수 설정
  (bind _asbp_gamemode (cast `/Game/Actor/BP_Gamemode` (`GameplayStatics.GetGameMode`)))
  (set `local.CurrentDifficulty` (`/Game/Actor/BP_Gamemode.DifficultyLevel` _asbp_gamemode))
  (set `local.CurrentMaxAlive` (+ (`self.BaseMaxAlive`) (* (`local.CurrentDifficulty`) (`self.MaxAlivePerDifficulty`))))
  (set `local.SpawnCount` (+ (`self. BaseSpawnCount`) (* (`local.CurrentDifficulty`) (`self.SpawnCountPerDifficulty`))))
  ; 현재 난이도에서 수용 가능한 수인지 체크
  (if (not (>= (`self.AliveEnemy`) (`local.CurrentMaxAlive`)))
    ; 스폰할 Enemy가 Pool에 있는 지 검사
    (for _array_element (`self.EnemyPool`)
      (`/Engine/EditorBlueprintResources/StandardMacros.IsValid` _array_element
        (:`Is Valid`
          (if (`Actor.bHidden` _array_element)
            (set `local.AvailableEnemy` _array_element)
            (break)))))
    ; Pool에 소환할 Enemy가 있다면 스폰
    (`/Engine/EditorBlueprintResources/StandardMacros.IsValid` (`local.AvailableEnemy`)
      (:`Is Valid`
        (`self.K2_SetActorLocation` _availableenemy (+ (`self.K2_GetActorLocation` (`self.PlayerRef`)) (`KismetMathLibrary.MakeVector` _returnvalue_x _returnvalue_y)) false true)
        (`self.SetActorHiddenInGame` _availableenemy false)
        (`self.SetActorTickEnabled` _availableenemy true)
        (`PrimitiveComponent.SetCollisionEnabled` (`Character.CapsuleComponent` _availableenemy) "QueryAndPhysics")
        (`/Game/Actor/Enemy/BP_Enemy.ResetEnemy` _availableenemy)
        (`/Engine/EditorBlueprintResources/StandardMacros.IncrementInt` (`self.AliveEnemy`))))))

(fn `UserConstructionScript`)