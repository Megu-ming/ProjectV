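; BP_Enemy is a pooled enemy that chases the player and deals damage on capsule hits with BP_Character.
; ResetEnemy restores HP and starts an AIMoveTo chase that re-issues itself on each success.
; Hit subtracts HP and at zero stops movement and plays a death montage.
; On blend out it returns to the pool by hiding, disabling tick and collision, and notifying SpawnerRef rather than being destroyed.
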(event `self.ReceiveBeginPlay`
  ; Initialize
  (set `self.CurrentHp` (`self.MaxHp`))
  (set `self.Target` (`GameplayStatics.GetPlayerCharacter` 0)))

(event `FollowPlayer`
  ; Chasing Player
  (`|AIMoveTo` self (0.0 0.0 0.0) (`self.Target`)
    (:`OnSuccess`
      (`self.FollowPlayer`))))

(event `Hit`
  (params (Damage :type "Float (double-precision)"))
  ; When enemy Hit by Player
  (bind _output_get (set `self.CurrentHp` (- (`self.CurrentHp`) Damage)))
  (if (<= _output_get 0.0)
    (`MovementComponent.StopMovementImmediately` (`self.CharacterMovement`))
    (`|PlayMontage` (`self.Mesh`) "/Game/Asset/GreystoneManny/Death_Montage.Death_Montage"
      (:`OnBlendOut`
        (`self.ReturnToPool`)))))

(event `ReturnToPool`
  (bind _spawnerref (`self.SpawnerRef`))
  ; When Enemy Died - Return Enemy to Pool
  (`Controller.StopMovement` (`AIBlueprintHelperLibrary.GetAIController` (`self.GetController`)))
  (`self.SetActorHiddenInGame` true)
  (`self.SetActorTickEnabled` false)
  (`PrimitiveComponent.SetCollisionEnabled` (`self.CapsuleComponent`) "NoCollision")
  (`/Engine/EditorBlueprintResources/StandardMacros.IsValid` _spawnerref
    (:`Is Valid`
      (`/Game/Actor/BP_EnemySpawner.OnEnemyReturned` _spawnerref))))

(event `ResetEnemy`
  ; Reset
  (set `self.CurrentHp` (`self.MaxHp`))
  (`self.FollowPlayer`))

(event `self.CapsuleComponent.OnComponentHit`
  (params (HitComponent :type "PrimitiveComponent Object Reference") (OtherActor :type "Actor Object Reference") (OtherComp :type "PrimitiveComponent Object Reference") (NormalImpulse :type "Vector Structure") (Hit :type "HitResult Structure (by ref)"))
  (bind _asbp_character (cast `/Game/Actor/BP_Character` OtherActor))
  (`/Game/Actor/BP_Character.HitByEnemy` _asbp_character (`self.AttackDamage`)))

(fn `UserConstructionScript`)