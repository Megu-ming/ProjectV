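; Player character with auto-attacking weapons, stat augments, and cooldown-gated damage intake that ends in a placeholder death message.
; BeginPlay copies base stats, equips the sword and starts a looping attack timer that calls the current weapon's Attack.
; EquipWeapon swaps a child actor's class and passes the weapon type to the anim Blueprint, with debug keys switching weapons.
; Augments multiply damage, move speed or attack speed, restarting the timer for the latter.
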(event Custom|HitByEnemy
  (params (Damage :type Float%20%28double-precision%29))
  ;[0.15 0.15 0.15 0.5] 피격판정
  (if (Variables|피격|GetCanbeHit)
    (Variables|피격|SetCanbeHit false)
    (Utilities|FlowControl|Sequence
      (:then_0
        (Utilities|Time|SetTimerbyFunctionName 0 "ResetHitEnable" (Variables|피격|GetHitCooldown) true))
      (:then_1
        (bind _output_get (Variables|상태|SetCurrentHp (- (Variables|상태|GetCurrentHp) Damage)))
        (if (<= _output_get 0.0)
          (CallFunction|Die))))))

(event Custom|Die
  ;[0.15 0.15 0.15 0.5] 사망 시 호출
  (Development|PrintText "Die"))

(event Custom|RefreshAutoAttackTimer
  ;[0.15 0.15 0.15 0.5] 자동공격 로직
  (Utilities|Time|ClearandInvalidateTimerbyHandle (Variables|Default|GetAutoAttackTimerHandler))
  (bind _returnvalue (Utilities|Time|SetTimerbyFunctionName 0 "AutoAttack" (Utilities|DPStoInterval (Variables|상태|GetAttackSpeed)) true))
  (Variables|Default|SetAutoAttackTimerHandler _returnvalue))

(event EventBeginPlay
  ;[0.15 0.15 0.15 0.5] 초기값 세팅
  (Variables|상태|SetCurrentHp (Variables|Status|GetMaxHp))
  (Variables|상태|SetAttackDamage (Variables|상태|GetBaseAttackDamage))
  (Variables|상태|SetAttackSpeed (Variables|상태|GetBaseAttackSpeed))
  (Variables|상태|SetMoveSpeed (Variables|상태|GetBaseMoveSpeed))
  (CallFunction|EquipWeapon "/Game/Actor/Weapon/BP_WeaponSword.BP_WeaponSword_C")
  ;[0.15 0.15 0.15 0.5] 자동공격 시작
  (CallFunction|RefreshAutoAttackTimer))

(event Input|KeyboardEvents|DebugKey1
  (params (Key :type Key%20Structure :default "None") (ActionValue :type Input%20Action%20Value%20Structure))
  (:Pressed
    (CallFunction|EquipWeapon "/Game/Actor/Weapon/BP_WeaponSword.BP_WeaponSword_C")))

(event Input|KeyboardEvents|DebugKey2
  (params (Key :type Key%20Structure :default "None") (ActionValue :type Input%20Action%20Value%20Structure))
  (:Pressed
    (CallFunction|EquipWeapon "/Game/Actor/Weapon/BP_WeaponPistol.BP_WeaponPistol_C")))

(event Input|KeyboardEvents|DebugKey3
  (params (Key :type Key%20Structure :default "None") (ActionValue :type Input%20Action%20Value%20Structure))
  (:Pressed
    (CallFunction|EquipWeapon "/Game/Actor/Weapon/BP_WeaponRifle.BP_WeaponRifle_C")))

(fn ConstructionScript)

(fn AutoAttack
  (bind _currentweapon (Variables|Default|GetCurrentWeapon))
  (Utilities|IsValid _currentweapon
    (:Is%20Valid
      (Default|Attack _currentweapon))))

(fn ResetHitEnable
  (Variables|피격|SetCanbeHit true))

(fn ApplyAugment
  (params (InData :type ST%20Augment%20Data%20Structure))
  (bind (_id _type _nametext _description _icon _value) (Utilities|Struct|BreakST_AugmentData InData))
  (LocalVariables|SetRate (+ (/ _value 1e+02) 1.0))
  (switch Utilities|FlowControl|Switch|SwitchonE_AugmentType _type
    (:NewEnumerator0
      (Variables|상태|SetAttackDamage (* (Variables|상태|GetAttackDamage) (LocalVariables|GetRate))))
    (:NewEnumerator1
      (bind _output_get (Variables|상태|SetMoveSpeed (* (Variables|상태|GetMoveSpeed) (LocalVariables|GetRate))))
      (Variables|/Script/Engine.CharacterMovementComponent|SetMaxWalkSpeed (Variables|Character|GetCharacterMovement) _output_get))
    (:NewEnumerator2
      (Variables|상태|SetAttackSpeed (* (Variables|상태|GetAttackSpeed) (LocalVariables|GetRate)))
      (CallFunction|RefreshAutoAttackTimer))))

(fn EquipWeapon
  (params (WeaponClass :type BP%20Weapon%20Base%20Class%20Reference))
  (bind _weaponchild (Variables|Default|GetWeaponChild))
  (ChildActorComponent|SetChildActorClass _weaponchild WeaponClass)
  (bind _asbp_weapon_base (Utilities|Casting|CastToBP_WeaponBase (Variables|/Script/Engine.ChildActorComponent|GetChildActor _weaponchild)))
  (bind _output_get (Variables|Default|SetCurrentWeapon _asbp_weapon_base))
  (Variables|/Game/Actor/Weapon/BP_WeaponBase.BP_WeaponBase_C|SetOwnerCharacter _output_get self)
  (bind _asabp_player (Utilities|Casting|CastToABP_Player (Components|SkeletalMesh|GetAnimInstance (Variables|Character|GetMesh))))
  (Variables|/Game/Animation/ABP_Player.ABP_Player_C|SetWeaponType _asabp_player (Variables|/Game/Actor/Weapon/BP_WeaponBase.BP_WeaponBase_C|GetWeaponType (Variables|Default|GetCurrentWeapon))))