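; Player controller that handles Enhanced Input movement and horizontal mouse look for the player character.
; On BeginPlay it adds the IMC_Move mapping context to the local player input subsystem.
; IA_Move drives the character along the controller's own forward and right vectors.
; IA_Look applies only yaw, scaled by MouseSensitivity, with no pitch handling.
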(event `self.ReceiveBeginPlay`
  (`EnhancedInputSubsystemInterface.AddMappingContext` (subsystem `EnhancedInputLocalPlayerSubsystem`) "/Game/Input/IMC_Move.IMC_Move" 0 (struct)))

(event `EnhancedInput|/Game/Input/IA_Move`
  (params (ActionValue :type "Vector2D Structure") (ElapsedSeconds :type "Float (double-precision)") (TriggeredSeconds :type "Float (double-precision)") (InputAction :type "InputAction Object Reference" :default "/Game/Input/IA_Move.IA_Move"))
  (bind _returnvalue (`GameplayStatics.GetPlayerCharacter` 0))
  (bind (_x _y) (`KismetMathLibrary.BreakVector2D` ActionValue))
  ; 입력(나중에 컨트롤러 쪽으로 이관)
  (:`Triggered`
    (`Pawn.AddMovementInput` _returnvalue (`self.GetActorForwardVector`) _x false)
    (`Pawn.AddMovementInput` _returnvalue (`self.GetActorRightVector`) _y false)))

(event `EnhancedInput|/Game/Input/IA_Look`
  (params (ActionValue :type "Float (double-precision)") (ElapsedSeconds :type "Float (double-precision)") (TriggeredSeconds :type "Float (double-precision)") (InputAction :type "InputAction Object Reference" :default "/Game/Input/IA_Look.IA_Look"))
  ; 입력(나중에 컨트롤러 쪽으로 이관)
  (:`Triggered`
    (`Pawn.AddControllerYawInput` (`GameplayStatics.GetPlayerCharacter` 0) (* (`KismetMathLibrary.BreakVector2D` (`KismetMathLibrary.Conv_DoubleToVector2D` ActionValue)) (`self.MouseSensitivity`)))))

(fn `UserConstructionScript`)